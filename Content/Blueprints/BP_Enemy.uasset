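; Enemy actor that chases its Target's ball, grabs it and heads back to its spawn position.
; Tick faces the ball, or the saved start once FoundBall is set, and does a swept move via GetNextPos, whose step calculation appears unconnected.
; ballTaked snaps the ball to the EsquiloV04 BallPos socket.
; Hit re-parents the ball to itself, enables its physics and destroys the enemy.
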(event Custom|ballTaked
  (params (Ball :type BP%20Ball%20Object%20Reference))
  (Transformation|AttachComponentToComponent (Variables|/Game/Blueprints/BP_Ball.BP_Ball_C|GetSphere (Variables|Default|GetTarget)) (Variables|Default|Getesquilo_v04) "BallPos" "SnapToTarget" "SnapToTarget" "KeepWorld" true)
  (Variables|Default|SetFoundBall true))

(event EventBeginPlay
  (Variables|Default|SetGotTheBallPos (Transformation|GetWorldLocation (Variables|Character|GetMesh))))

(event EventTick
  (params (DeltaSeconds :type Float%20%28single-precision%29))
  (bind _mesh (Variables|Character|GetMesh))
  (bind _target (Variables|Default|GetTarget))
  (Development|PrintString (Utilities|GetDisplayName _target))
  (Variables|Default|SetDeltaTime DeltaSeconds)
  (if (Variables|Default|GetFoundBall)
    (Variables|Default|SetEndPos (Variables|Default|GetGotTheBallPos))
    (else
      (bind _output_get (Variables|Default|SetEndPos (Transformation|GetWorldLocation (Variables|/Game/Blueprints/BP_Ball.BP_Ball_C|GetSphere _target))))))
  (bind _output_get_2 (Variables|Default|SetStartPos (Transformation|GetWorldLocation (Variables|Character|GetMesh))))
  (Transformation|SetRelativeLocationAndRotation _mesh "0, 0, 0" (Math|Rotator|FindLookatRotation _output_get_2 (Variables|Default|GetEndPos)) true false)
  (Transformation|SetWorldLocation _mesh (+ (Utilities|GetNextPos _output_get_2 _output_get (Variables|Default|GetSpeed) 0.09) "0,0.000000,10.000000") true false))

(event Collision|EventHit
  (params (MyComp :type Primitive%20Component%20Object%20Reference) (Other :type Actor%20Object%20Reference) (OtherComp :type Primitive%20Component%20Object%20Reference) (bSelfMoved :type Boolean) (HitLocation :type Vector :default "0, 0, 0") (HitNormal :type Vector :default "0, 0, 0") (NormalImpulse :type Vector :default "0, 0, 0") (Hit :type Hit%20Result%20Structure%20%28by%20ref%29))
  (bind _target (Variables|Default|GetTarget))
  (bind _sphere (Variables|/Game/Blueprints/BP_Ball.BP_Ball_C|GetSphere _target))
  (Transformation|AttachComponentToComponent (Variables|/Game/Blueprints/BP_Ball.BP_Ball_C|GetSphere _target) _sphere "BallPos" "KeepWorld" "KeepWorld" "KeepWorld" true)
  (Physics|SetSimulatePhysics _sphere true)
  (Actor|DestroyActor))

(fn ConstructionScript)