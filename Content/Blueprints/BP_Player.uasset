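; Player Blueprint for a gyro-aimed shooter that creates the HUD and fires projectiles along the camera's view.
; Motion rotation rate drives yaw and pitch each Tick alongside axis input, with initial pitch calibrated from device tilt.
; Holding Fire calls GunShot from both a looping timer and a Tick accumulator, with hover time feeding GetCurrentFireRate, whose formula is unconnected.
; Shots build heat up to a firing cap; release starts a cooldown timer.
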(event Custom|GunShot
  (bind _camera (Variables|Default|GetCamera))
  (bind _maxheatlevel (Variables|Gun|GetMaxHeatLevel))
  (bind _returnvalue (Transformation|GetWorldRotation _camera))
  ;[1 1 1] Gun
  (Variables|Gun|SetCurrentFireRate (Utilities|GetCurrentFireRate (Variables|Gun|GetHoverTime)))
  (if (< (Variables|Gun|GetHeatLevel) _maxheatlevel)
    (Game|SpawnActorfromClass "/Game/Blueprints/BP_Projectile.BP_Projectile_C" (Math|Transform|MakeTransform (+ (+ (Transformation|GetWorldLocation (Variables|Default|GetGun)) "0, 0,200.000000") (Math|Vector|RotateVector "150.000000, 0, 0" _returnvalue)) _returnvalue "0.500000,0.500000,0.500000") "AdjustIfPossibleButDontSpawnIfColliding" 0 0)
    (bind _result (Math|Float|IncrementFloat (Variables|Gun|GetHeatLevel))
      (:%20%20
        (Variables|Gun|SetHeatLevel _result)))
    (else
      (Variables|Gun|SetHeatLevel _maxheatlevel))))

(event Custom|Calibrate
  (bind _returnvalue (Game|GetPlayerController 0))
  (bind (_tilt _rotationrate) (Class|PlayerController|GetInputMotionState _returnvalue))
  (bind _returnvalue_2 (Math|Float|Absolute(Float) (.x _tilt)))
  ;[1 1 1] Moviment
  (Class|KismetInputLibrary|CalibrateTilt)
  (Variables|/Script/Engine.PlayerController|SetInputPitchScale (Game|GetPlayerController 0) 1.0)
  (Utilities|FlowControl|Delay 0.25)
  (if (> _returnvalue_2 1.5)
    (bind _newangle (CallFunction|CorrectDiffTiltValue _returnvalue_2))
    (Pawn|Input|AddControllerPitchInput _newangle)
    (else
      (bind _newangle_2 (CallFunction|CorrectDiffTiltValue _returnvalue_2))
      (Pawn|Input|AddControllerPitchInput (* _newangle_2 -1.0)))))

(event Custom|ClearHeatLevel
  ;[1 1 1] Gun
  (if (> (Variables|Gun|GetHeatLevel) 0.0)
    (bind _result (Math|Float|DecrementFloat (Variables|Gun|GetHeatLevel))
      (:%20%20
        (Variables|Gun|SetHeatLevel _result)))))

(event Custom|CountHoverTime
  (params (DeltaSeconds :type Float%20%28single-precision%29))
  ;[1 1 1] Touch Pressed
  (bind _output_get (Variables|Gun|SetHoverTime (Math|Float|Clamp(Float) (+ (* (Variables|Gun|GetHoverTimeDirection) DeltaSeconds) (Variables|Gun|GetHoverTime)) 0.0 (Variables|Gun|GetMaxHoverTIme))))
  (if (== (Variables|Gun|GetHoverTimeDirection) 1)
    (bind _output_get_2 (Variables|Gun|SetFireRateTick (+ DeltaSeconds (Variables|Gun|GetFireRateTick))))
    (Development|PrintString (Utilities|String|ToString(Float) 0.0) true true "(R=0.000000,G=0.660000,B=1.000000,A=1.000000)" 0.0)
    (if (>= _output_get_2 (Utilities|GetCurrentFireRate _output_get))
      (CallFunction|GunShot)
      (Variables|Gun|SetFireRateTick 0.0))))

(event EventBeginPlay
  (CallFunction|Calibrate)
  (bind _returnvalue (UserInterface|CreateWidget "/Game/Blueprints/UMG/Widget_HUD.Widget_HUD_C" (Game|GetPlayerController 0)))
  (bind _output_get (Variables|Default|SetHUD _returnvalue))
  (UserInterface|Viewport|AddtoViewport _output_get 0))

(event EventTick
  (params (DeltaSeconds :type Float%20%28single-precision%29))
  (bind _returnvalue (Game|GetPlayerController 0))
  (bind (_tilt _rotationrate) (Class|PlayerController|GetInputMotionState _returnvalue))
  ;[1 1 1] Moviment
  (CallFunction|CountHoverTime DeltaSeconds)
  (Pawn|Input|AddControllerYawInput (* (.y _rotationrate) -1.0))
  (Pawn|Input|AddControllerPitchInput (* (.x _rotationrate) -1.0)))

(event Input|ActionEvents|InputActionFire
  (params (Key :type Key%20Structure :default "AnyKey"))
  ;[1 1 1] Gun
  (:Pressed
    (Variables|Gun|SetHoverTimeDirection 1)
    (Utilities|Time|ClearandInvalidateTimerbyHandle (Variables|Gun|GetClearHeatTimer))
    (bind _returnvalue (Utilities|Time|SetTimerbyFunctionName 0 "GunShot" (Variables|Gun|GetCurrentFireRate) true))
    (Variables|Gun|SetFireRateTimer _returnvalue))
  (:Released
    (Variables|Gun|SetHoverTimeDirection -1)
    (Utilities|Time|ClearandInvalidateTimerbyHandle (Variables|Gun|GetFireRateTimer))
    (bind _returnvalue_2 (Utilities|Time|SetTimerbyFunctionName 0 "ClearHeatLevel" (Variables|Gun|GetClearHeatRate) true))
    (Variables|Gun|SetClearHeatTimer _returnvalue_2)))

(event Input|AxisEvents|InputAxisTurn
  (params (AxisValue :type Float%20%28single-precision%29))
  ;[1 1 1] Moviment
  (Pawn|Input|AddControllerYawInput AxisValue))

(event Input|AxisEvents|InputAxisLookUp
  (params (AxisValue :type Float%20%28single-precision%29))
  ;[1 1 1] Moviment
  (Pawn|Input|AddControllerPitchInput AxisValue))

(fn ConstructionScript)

(fn CorrectDiffTiltValue
  (params (CurrentTilt :type Float%20%28single-precision%29))
  (return (Math|Float|Absolute(Float) (* (- (LocalVariables|GetMaxTilt) CurrentTilt) (LocalVariables|GetMaxAngle)))))