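; Projectile actor that knocks components tagged Ball on impact.
; On hit, it adds an impulse to such a component at the projectile's location, using its own velocity scaled by HitImpulse.
; After any hit, it disables collision on Sphere, hides Collision and its children, then destroys itself after a short delay.
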(event Collision|EventHit
  (params (MyComp :type Primitive%20Component%20Object%20Reference) (Other :type Actor%20Object%20Reference) (OtherComp :type Primitive%20Component%20Object%20Reference) (bSelfMoved :type Boolean) (HitLocation :type Vector :default "0, 0, 0") (HitNormal :type Vector :default "0, 0, 0") (NormalImpulse :type Vector :default "0, 0, 0") (Hit :type Hit%20Result%20Structure%20%28by%20ref%29))
  (if (Components|ComponentHasTag OtherComp "Ball")
    (Physics|AddImpulseatLocation OtherComp (* (Transformation|GetVelocity) (Variables|Default|GetHitImpulse)) (Transformation|GetActorLocation) "None"))
  (Collision|SetCollisionEnabled (Variables|Default|GetSphere) "NoCollision")
  (Rendering|SetVisibility (Variables|Default|GetCollision) false true)
  (Utilities|FlowControl|Delay 0.2)
  (Actor|DestroyActor))

(fn ConstructionScript)